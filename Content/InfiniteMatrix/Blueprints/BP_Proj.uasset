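; BP_Proj is a projectile actor that travels straight along world +X and destroys itself after covering a set distance.
; BeginPlay turns Distance into an absolute X limit from the spawn location and sets a default ForwardSpeed.
; Tick moves the actor by a frame-rate independent world offset until it passes that limit.
; SetForwardSpeed lets callers change the speed, though BeginPlay overwrites any value set earlier.
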(event EventBeginPlay
  (Variables|Default|SetDistance (+ (.x (.location (Transformation|GetActorTransform))) (Variables|Default|GetDistance)))
  (Variables|Default|SetForward%20Speed 3e+03))

(event Collision|EventActorBeginOverlap
  (params (OtherActor :type Actor%20Object%20Reference)))

(event EventTick
  (params (DeltaSeconds :type Float%20%28single-precision%29))
  (if (> (.x (.location (Transformation|GetActorTransform))) (Variables|Default|GetDistance))
    (Actor|DestroyActor)
    (else
      (Transformation|AddActorWorldOffset (Math|Vector|MakeVector (* (Variables|Default|GetForward%20Speed) DeltaSeconds) 0.0 0.0)))))

(fn ConstructionScript)

(fn SetForwardSpeed
  (params (NewParam :type Float%20%28single-precision%29))
  (Variables|Default|SetForward%20Speed NewParam))